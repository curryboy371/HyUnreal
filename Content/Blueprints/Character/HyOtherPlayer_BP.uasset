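; Character Blueprint for another player, which sets up locomotion animation and movement tuning on spawn.
; BeginPlay links the unarmed linked anim layer class to the mesh and sets the state to Jogging.
; It looks up that state's movement options in a map, copies speed, acceleration and braking settings to CharacterMovement through Test, then notifies the AnimInstance of the state via SwitchMoveMessage.
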(event `self.ReceiveBeginPlay`
  (`SkeletalMeshComponent.LinkAnimClassLayers` (`self.Mesh`) "/Game/Blueprints/Animation/Layer/ABP_UnArmed.ABP_UnArmed_C")
  (bind _output_get (set `self.CharacterState` "Jogging"))
  (bind (_value _returnvalue) (`BlueprintMapLibrary.Map_Find` (`self.CharacterMoveOptionMap`) _output_get))
  (if _returnvalue
    (`self.Test` _value)
    (message `/Game/Blueprints/Interfaces/BPI_Animation.SwitchMove` (`SkeletalMeshComponent.GetAnimInstance` (`self.Mesh`)) (`self.CharacterState`))))

(fn `Test`
  (params (NewParam :type "CharacterMoveOption Structure"))
  (bind (_maxwalkspeed _maxacceleration _brakingdeceleration _brakingfrictionfactor _brakingfriction _useseparatebrakingfriction) (break `CharacterMoveOption` NewParam))
  (bind _charactermovement (`self.CharacterMovement`))
  (set `CharacterMovementComponent.MaxWalkSpeed` _maxwalkspeed _charactermovement)
  (set `CharacterMovementComponent.MaxAcceleration` _maxacceleration _charactermovement)
  (set `CharacterMovementComponent.BrakingDecelerationWalking` _brakingdeceleration _charactermovement)
  (set `CharacterMovementComponent.BrakingFrictionFactor` _brakingfrictionfactor _charactermovement)
  (set `CharacterMovementComponent.BrakingFriction` _brakingfriction _charactermovement)
  (set `CharacterMovementComponent.bUseSeparateBrakingFriction` _useseparatebrakingfriction _charactermovement))

(fn `UserConstructionScript`)