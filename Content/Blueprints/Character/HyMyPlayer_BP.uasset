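; Player character Blueprint that switches weapon animation sets and movement states, apparently as a locomotion test setup.
; Test inputs set the equipped weapon state and link the unarmed, rifle or pistol anim class layer to the mesh.
; Skill inputs pick Walking or Jogging (the default), apply that state's CharacterMovement settings from a map, and notify the anim instance.
; Debug keys toggle slow-motion time dilation; an equip-action message is left unconnected.
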(event `self.ReceiveBeginPlay`
  (`SkeletalMeshComponent.LinkAnimClassLayers` (`self.Mesh`) "/Game/Blueprints/Animation/Layer/ABP_UnArmed.ABP_UnArmed_C")
  (bind _output_get (set `self.CharacterState` "Jogging"))
  (bind (_value _returnvalue) (`BlueprintMapLibrary.Map_Find` (`self.CharacterMoveOptionMap`) _output_get))
  (if _returnvalue
    (`self.Test` _value)
    (message `/Game/Blueprints/Interfaces/BPI_Animation.SwitchMove` (`SkeletalMeshComponent.GetAnimInstance` (`self.Mesh`)) (`self.CharacterState`))))

(event `EnhancedInput|/Game/Blueprints/Input/Action/IA_Test1`
  (params (ActionValue :type Boolean) (ElapsedSeconds :type "Float (double-precision)") (TriggeredSeconds :type "Float (double-precision)") (InputAction :type "InputAction Object Reference" :default "/Game/Blueprints/Input/Action/IA_Test1.IA_Test1"))
  (:`Started`
    (set `self.EquippedWeaponState` "UnArmed")
    (`SkeletalMeshComponent.LinkAnimClassLayers` (`self.Mesh`) "/Game/Blueprints/Animation/Layer/ABP_UnArmed.ABP_UnArmed_C")))

(event `EnhancedInput|/Game/Blueprints/Input/Action/IA_Test2`
  (params (ActionValue :type Boolean) (ElapsedSeconds :type "Float (double-precision)") (TriggeredSeconds :type "Float (double-precision)") (InputAction :type "InputAction Object Reference" :default "/Game/Blueprints/Input/Action/IA_Test2.IA_Test2"))
  (:`Started`
    (set `self.EquippedWeaponState` "Rifle")
    (`SkeletalMeshComponent.LinkAnimClassLayers` (`self.Mesh`) "/Game/Blueprints/Animation/Layer/ABP_Rifle.ABP_Rifle_C")))

(event `EnhancedInput|/Game/Blueprints/Input/Action/IA_Test3`
  (params (ActionValue :type Boolean) (ElapsedSeconds :type "Float (double-precision)") (TriggeredSeconds :type "Float (double-precision)") (InputAction :type "InputAction Object Reference" :default "/Game/Blueprints/Input/Action/IA_Test3.IA_Test3"))
  (:`Started`
    (set `self.EquippedWeaponState` "Pistol")
    (`SkeletalMeshComponent.LinkAnimClassLayers` (`self.Mesh`) "/Game/Blueprints/Animation/Layer/ABP_Pistol.ABP_Pistol_C")))

(event `EnhancedInput|/Game/Blueprints/Input/Action/IA_Skill1`
  (params (ActionValue :type Boolean) (ElapsedSeconds :type "Float (double-precision)") (TriggeredSeconds :type "Float (double-precision)") (InputAction :type "InputAction Object Reference" :default "/Game/Blueprints/Input/Action/IA_Skill1.IA_Skill1"))
  (:`Started`
    (bind _output_get (set `self.CharacterState` "Walking"))
    (bind (_value _returnvalue) (`BlueprintMapLibrary.Map_Find` (`self.CharacterMoveOptionMap`) _output_get))
    (if _returnvalue
      (`self.Test` _value)
      (message `/Game/Blueprints/Interfaces/BPI_Animation.SwitchMove` (`SkeletalMeshComponent.GetAnimInstance` (`self.Mesh`)) (`self.CharacterState`) :!label _label))))

(event `EnhancedInput|/Game/Blueprints/Input/Action/IA_Skill2`
  (params (ActionValue :type Boolean) (ElapsedSeconds :type "Float (double-precision)") (TriggeredSeconds :type "Float (double-precision)") (InputAction :type "InputAction Object Reference" :default "/Game/Blueprints/Input/Action/IA_Skill2.IA_Skill2"))
  (:`Started`
    (bind _output_get (set `self.CharacterState` "Jogging"))
    (bind (_value _returnvalue) (`BlueprintMapLibrary.Map_Find` (`self.CharacterMoveOptionMap`) _output_get))
    (if _returnvalue
      (`self.Test` _value)
      (goto _label))))

(event `Key|Subtract`
  (params (Key :type "Key Structure"))
  (:`Pressed`
    (`GameplayStatics.SetGlobalTimeDilation` 0.1)))

(event `Key|Add`
  (params (Key :type "Key Structure"))
  (:`Pressed`
    (`GameplayStatics.SetGlobalTimeDilation` 1.0)))

(fn `Test`
  (params (NewParam :type "CharacterMoveOption Structure"))
  (bind (_maxwalkspeed _maxacceleration _brakingdeceleration _brakingfrictionfactor _brakingfriction _useseparatebrakingfriction) (break `CharacterMoveOption` NewParam))
  (bind _charactermovement (`self.CharacterMovement`))
  (set `CharacterMovementComponent.MaxWalkSpeed` _maxwalkspeed _charactermovement)
  (set `CharacterMovementComponent.MaxAcceleration` _maxacceleration _charactermovement)
  (set `CharacterMovementComponent.BrakingDecelerationWalking` _brakingdeceleration _charactermovement)
  (set `CharacterMovementComponent.BrakingFrictionFactor` _brakingfrictionfactor _charactermovement)
  (set `CharacterMovementComponent.BrakingFriction` _brakingfriction _charactermovement)
  (set `CharacterMovementComponent.bUseSeparateBrakingFriction` _useseparatebrakingfriction _charactermovement))

(fn `UserConstructionScript`)